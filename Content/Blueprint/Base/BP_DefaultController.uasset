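; BP_DefaultController is a controller that lets the player position and submit cargo with the keyboard.
; It selects the first cargo from the game mode's CurrentCargoActors on BeginPlay, reselecting on WASD if invalid.
; WASD shifts CurPos by one unit, Q/E rotate and Z toggles IsLaid.
; Space submits through the game mode; success advances the wrapping selection and updates the HUD name from DT_CargoInfo.
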(event Custom|SelectNewCargo
  (bind _cargo_game_mode (CallFunction|GetCargoGameMode self))
  (bind (_array_element _array_index) (Utilities|Array|ForEachLoopwithBreak (Variables|/Game/Blueprint/Base/BP_CargoGameMode.BP_CargoGameMode_C|GetCurrentCargoActors _cargo_game_mode) :!label _label)
    (:LoopBody
      (Variables|Default|SetSelectedCargo _array_element)
      (Variables|Default|SetSelectedIndex _array_index)
      (goto _label Break))))

(event Custom|SelectNextCargo
  (bind _cargo_game_mode (CallFunction|GetCargoGameMode self))
  (bind (_array_element _array_index) (Utilities|Array|ForEachLoopwithBreak (Variables|/Game/Blueprint/Base/BP_CargoGameMode.BP_CargoGameMode_C|GetCurrentCargoActors _cargo_game_mode) :!label _label)
    (:LoopBody
      (if (== _array_index (select (>= (+ (Variables|Default|GetSelectedIndex) 1) (Utilities|Array|Length (Variables|/Game/Blueprint/Base/BP_CargoGameMode.BP_CargoGameMode_C|GetCurrentCargoActors _cargo_game_mode))) 0 (+ (Variables|Default|GetSelectedIndex) 1)))
        (Variables|Default|SetSelectedCargo _array_element)
        (Variables|Default|SetSelectedIndex (select (>= (+ (Variables|Default|GetSelectedIndex) 1) (Utilities|Array|Length (Variables|/Game/Blueprint/Base/BP_CargoGameMode.BP_CargoGameMode_C|GetCurrentCargoActors _cargo_game_mode))) 0 (+ (Variables|Default|GetSelectedIndex) 1)))
        (goto _label Break)))))

(event EventBeginPlay
  (|CallParentFunction)
  (CallFunction|SelectNewCargo))

(event Input|KeyboardEvents|W
  (params (Key :type Key%20Structure :default "None"))
  (bind _selectedcargo (Variables|Default|GetSelectedCargo))
  (:Pressed
    (Utilities|IsValid _selectedcargo
      (:Is%20Valid
        _)
      (:Is%20Not%20Valid
        (CallFunction|SelectNewCargo)))
    (Variables|/Game/Blueprint/Base/BP_CargoBase.BP_CargoBase_C|SetCurPos _selectedcargo (+ (Variables|/Game/Blueprint/Base/BP_CargoBase.BP_CargoBase_C|GetCurPos _selectedcargo) "1.000000,0.000000,0.000000"))))

(event Input|KeyboardEvents|D
  (params (Key :type Key%20Structure :default "None"))
  (bind _selectedcargo (Variables|Default|GetSelectedCargo))
  (:Pressed
    (Utilities|IsValid _selectedcargo
      (:Is%20Valid
        _)
      (:Is%20Not%20Valid
        (CallFunction|SelectNewCargo)))
    (Variables|/Game/Blueprint/Base/BP_CargoBase.BP_CargoBase_C|SetCurPos _selectedcargo (+ (Variables|/Game/Blueprint/Base/BP_CargoBase.BP_CargoBase_C|GetCurPos _selectedcargo) "0.000000,1.000000,0.000000"))))

(event Input|KeyboardEvents|A
  (params (Key :type Key%20Structure :default "None"))
  (bind _selectedcargo (Variables|Default|GetSelectedCargo))
  (:Pressed
    (Utilities|IsValid _selectedcargo
      (:Is%20Valid
        _)
      (:Is%20Not%20Valid
        (CallFunction|SelectNewCargo)))
    (Variables|/Game/Blueprint/Base/BP_CargoBase.BP_CargoBase_C|SetCurPos _selectedcargo (+ (Variables|/Game/Blueprint/Base/BP_CargoBase.BP_CargoBase_C|GetCurPos _selectedcargo) "0.000000,-1.000000,0.000000"))))

(event Input|KeyboardEvents|S
  (params (Key :type Key%20Structure :default "None"))
  (bind _selectedcargo (Variables|Default|GetSelectedCargo))
  (:Pressed
    (Utilities|IsValid _selectedcargo
      (:Is%20Valid
        _)
      (:Is%20Not%20Valid
        (CallFunction|SelectNewCargo)))
    (Variables|/Game/Blueprint/Base/BP_CargoBase.BP_CargoBase_C|SetCurPos _selectedcargo (+ (Variables|/Game/Blueprint/Base/BP_CargoBase.BP_CargoBase_C|GetCurPos _selectedcargo) "-1.000000,0.000000,0.000000"))))

(event Input|KeyboardEvents|SpaceBar
  (params (Key :type Key%20Structure :default "None"))
  (:Pressed
    (bind _cargo_game_mode (CallFunction|GetCargoGameMode self))
    (bind _issuccess (Default|SumitCargotoPos _cargo_game_mode (Variables|Default|GetSelectedIndex)))
    (if _issuccess
      (CallFunction|SelectNextCargo)
      (bind _returnvalue (Utilities|GetDataTableRow "/Game/Blueprint/DataTable/DT_CargoInfo.DT_CargoInfo" (Variables|/Game/Blueprint/Base/BP_CargoBase.BP_CargoBase_C|GetCargoInfoRowName (Variables|Default|GetSelectedCargo)))
        (:then
          (Default|SetCurrentCargoName (Variables|/Game/Blueprint/Base/BP_CargoGameMode.BP_CargoGameMode_C|GetCargoHUDWidget _cargo_game_mode) (Utilities|Text|ToText(String) (Utilities|Struct|BreakSCargoInfo _returnvalue))))))))

(event Input|KeyboardEvents|Q
  (params (Key :type Key%20Structure :default "None"))
  (bind _selectedcargo (Variables|Default|GetSelectedCargo))
  (:Pressed
    (Utilities|IsValid _selectedcargo
      (:Is%20Valid
        (Default|Rotation _selectedcargo true)))))

(event Input|KeyboardEvents|E
  (params (Key :type Key%20Structure :default "None"))
  (bind _selectedcargo (Variables|Default|GetSelectedCargo))
  (:Pressed
    (Utilities|IsValid _selectedcargo
      (:Is%20Valid
        (Default|Rotation _selectedcargo false)))))

(event Input|KeyboardEvents|Z
  (params (Key :type Key%20Structure :default "None"))
  (bind _selectedcargo (Variables|Default|GetSelectedCargo))
  (:Pressed
    (Utilities|IsValid _selectedcargo
      (:Is%20Valid
        (Variables|/Game/Blueprint/Base/BP_CargoBase.BP_CargoBase_C|SetIsLaid _selectedcargo (not (Variables|/Game/Blueprint/Base/BP_CargoBase.BP_CargoBase_C|GetIsLaid _selectedcargo)))))))

(fn ConstructionScript)