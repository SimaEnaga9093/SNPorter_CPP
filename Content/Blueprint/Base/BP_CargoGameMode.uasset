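; Game mode for a cargo-packing game that sets up a 3D block grid and tracks which cargo occupies each cell.
; On BeginPlay it builds a debug-drawn cell map sized from a data table, centers the pawn, spawns cargo actors and shows the HUD.
; SumitCargoToPos rotates a cargo's block offsets, rejects cells held by other cargo, otherwise records its index.
; Cells outside the grid do not block placement, and previously held cells are not cleared.
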(event EventBeginPlay
  (bind _cargosize (Variables|Default|GetCargoSize))
  (|CallParentFunction)
  (Utilities|FlowControl|Sequence
    (:then_0
      (bind _returnvalue (Utilities|GetDataTableRow "/Game/Blueprint/DataTable/DT_Float.DT_Float" "Block_OffsetSize")
        (:then
          (Variables|Default|SetBlockOffsetSize (Utilities|Struct|BreakSFloat _returnvalue)))))
    (:then_1
      (for _index (range 0 (- (Math|Float|Truncate (.x _cargosize)) 1))
        (for _index_2 (range 0 (- (Math|Float|Truncate (.y _cargosize)) 1))
          (for _index_3 (range 0 (- (Math|Float|Truncate (.z _cargosize)) 1))
            (Rendering|Debug|DrawDebugBox (Math|Vector|MakeVector (* _index (Variables|Default|GetBlockOffsetSize)) (* _index_2 (Variables|Default|GetBlockOffsetSize)) (* _index_3 (Variables|Default|GetBlockOffsetSize))) (* (Class|KismetMathLibrary|VectorOne) (Variables|Default|GetBlockOffsetSize) 0.5) "(R=0.000000,G=0.000000,B=0.000000,A=1.000000)" "0, 0, 0" 999.0 0.5)
            (Utilities|Map|Add (Variables|Default|GetLoadedCargoInfo) (Math|Vector|MakeVector (Math|Conversions|ToFloat(Integer) _index) (Math|Conversions|ToFloat(Integer) _index_2) (Math|Conversions|ToFloat(Integer) _index_3)) -1)))))
    (:then_2
      (Transformation|Teleport (Game|Player|GetPlayerPawn 0) (* (- (Variables|Default|GetCargoSize) (Class|KismetMathLibrary|VectorOne)) (Variables|Default|GetBlockOffsetSize) 0.5) "0, 0, 0"))
    (:then_3
      (for _array_element (Variables|Default|GetCurrentCargos)
        (bind _returnvalue_2 (Game|SpawnActorfromClass "/Game/Blueprint/Base/BP_CargoBase.BP_CargoBase_C" (Math|Transform|MakeTransform "0, 0, 0") "AlwaysSpawn" "MultiplyWithRoot" 0 0))
        (Utilities|Array|Add (Variables|Default|GetCurrentCargoActors) _returnvalue_2)))
    (:then_4
      (bind _returnvalue_3 (UserInterface|CreateWidget "/Game/Blueprint/Widget/WBP_CargoHUD.WBP_CargoHUD_C" (Game|GetPlayerController 0)))
      (UserInterface|Viewport|AddtoViewport _returnvalue_3 0)
      (Variables|Default|SetCargoHUDWidget _returnvalue_3))))

(fn ConstructionScript)

(fn SumitCargotoPos
  (params (CargoIndex :type Integer))
  (bind _currentcargoactors (Variables|Default|GetCurrentCargoActors))
  (bind _output (Utilities|Array|Get(acopy) _currentcargoactors CargoIndex))
  (bind _curpos (Variables|/Game/Blueprint/Base/BP_CargoBase.BP_CargoBase_C|GetCurPos _output))
  (Development|PrintText (Utilities|Text|FormatText "Cur index {i}" CargoIndex))
  (bind _rotation (Default|GetForwardRotation _output))
  (bind _currentposinfos (Default|GetCurrentCargoInfo _output))
  (for _array_element _currentposinfos
    (Development|PrintText (Utilities|Text|FormatText "{tf} {at} {what}" (.ReturnValue (Utilities|Map|Find (Variables|Default|GetLoadedCargoInfo) (+ (Math|Vector|RotateVector _array_element _rotation) _curpos))) (Utilities|String|ToString(Vector) (+ (Math|Vector|RotateVector _array_element _rotation) _curpos)) (.Value (Utilities|Map|Find (Variables|Default|GetLoadedCargoInfo) (+ (Math|Vector|RotateVector _array_element _rotation) _curpos)))))
    (if (Math|Boolean|ANDBoolean (!= (.Value (Utilities|Map|Find (Variables|Default|GetLoadedCargoInfo) (+ (Math|Vector|RotateVector _array_element _rotation) _curpos))) CargoIndex) (.ReturnValue (Utilities|Map|Find (Variables|Default|GetLoadedCargoInfo) (+ (Math|Vector|RotateVector _array_element _rotation) _curpos))) (!= (.Value (Utilities|Map|Find (Variables|Default|GetLoadedCargoInfo) (+ (Math|Vector|RotateVector _array_element _rotation) _curpos))) -1))
      (return false)))
  (for _array_element_2 _currentposinfos
    (Utilities|Map|Add (Variables|Default|GetLoadedCargoInfo) (+ (Math|Vector|RotateVector _array_element_2 _rotation) _curpos) CargoIndex)
    (Rendering|Debug|DrawDebugBox (* (+ (Math|Vector|RotateVector _array_element_2 _rotation) _curpos) (Variables|Default|GetBlockOffsetSize)) (* (Class|KismetMathLibrary|VectorOne) (Variables|Default|GetBlockOffsetSize) 0.4) "(R=0.000000,G=1.000000,B=0.944969,A=1.000000)" "0, 0, 0" 3.0 1.0))
  (return true))