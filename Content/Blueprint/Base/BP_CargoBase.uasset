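; Base Blueprint for a grid-placed cargo piece made of blocks, with a position, a four-step yaw rotation and an optional laid shape.
; BeginPlay loads the block size and the piece's row of block offsets from data tables.
; Tick rotates the active offsets and draws them as debug boxes, red when selected in the cargo controller and yellow otherwise, plus a forward arrow.
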(event EventBeginPlay
  (|CallParentFunction)
  (bind _returnvalue (Utilities|GetDataTableRow "/Game/Blueprint/DataTable/DT_Float.DT_Float" "Block_OffsetSize")
    (:then
      (Variables|Default|SetBlockOffsetSize (Utilities|Struct|BreakSFloat _returnvalue))
      (bind _returnvalue_2 (Utilities|GetDataTableRow "/Game/Blueprint/DataTable/DT_CargoInfo.DT_CargoInfo" (Variables|Default|GetCargoInfoRowName))
        (:then
          (Variables|Default|SetCargoInfo _returnvalue_2))))))

(event EventTick
  (params (DeltaSeconds :type Float%20%28single-precision%29))
  (bind _blockoffsetsize (Variables|Default|GetBlockOffsetSize))
  (bind _curpos (Variables|Default|GetCurPos))
  (bind _returnvalue (* _curpos _blockoffsetsize))
  (|CallParentFunction DeltaSeconds)
  (if (!= (Variables|Default|GetCargoInfoRowName) "")
    (bind (_vector _rotation) (CallFunction|GetForwardRotation))
    (bind _currentposinfos (CallFunction|GetCurrentCargoInfo))
    (for _array_element _currentposinfos
      (bind _cargo_controller (CallFunction|GetCargoController self))
      (Rendering|Debug|DrawDebugBox (* (+ (Math|Vector|RotateVector _array_element _rotation) (Variables|Default|GetCurPos)) (Variables|Default|GetBlockOffsetSize)) (* (Class|KismetMathLibrary|VectorOne) (Variables|Default|GetBlockOffsetSize) 0.5) (select (== self (Variables|/Game/Blueprint/Base/BP_DefaultController.BP_DefaultController_C|GetSelectedCargo _cargo_controller)) "(R=1.000000,G=0.000000,B=0.000000,A=1.000000)" "(R=1.000000,G=1.000000,B=0.000000,A=1.000000)") "0, 0, 0" 0.11 1.0))
    (Rendering|Debug|DrawDebugArrow _returnvalue (+ _returnvalue (* _vector 5e+01)) 1e+01 "(R=0.000000,G=1.000000,B=0.000000,A=1.000000)" 0.111 5.0)))

(fn ConstructionScript)

(fn Rotation
  (params (IsLeft :type Boolean))
  (bind _output_get (Variables|Default|SetCurRot (+ (Variables|Default|GetCurRot) (select IsLeft 1 -1))))
  (if (> _output_get 3)
    (Variables|Default|SetCurRot 0)
    (elif (< _output_get 0)
      (Variables|Default|SetCurRot 3))))

(fn GetCurrentCargoInfo
  (bind _cargoinfo (Variables|Default|GetCargoInfo))
  (bind (_posinfos _poslaidinfos) (Utilities|Struct|BreakSCargoInfo _cargoinfo))
  (return (select (and (Utilities|Array|IsNotEmpty _poslaidinfos) (Variables|Default|GetIsLaid)) _poslaidinfos _posinfos)))

(fn GetForwardRotation
  (bind _currot (Variables|Default|GetCurRot))
  (bind _returnvalue (* _currot -90))
  (bind _returnvalue_2 (Math|Rotator|MakeRotator 0.0 0.0 _returnvalue))
  (return (Math|Vector|GetForwardVector _returnvalue_2) _returnvalue_2))